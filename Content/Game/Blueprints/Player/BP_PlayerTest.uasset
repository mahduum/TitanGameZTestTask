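; Test player Blueprint for click-selecting agents and buildings and assigning one to the other.
; BeginPlay adds the default Enhanced Input context; left click traces under the cursor and stores the tagged agent or building hit.
; Once both are set it calls Assign on the agent; clicking anything else resets that agent's assignment blackboard keys and clears both selections.
; Jump input and clicks print debug text; a disconnected chain of agent toggle calls never runs.
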(event Input|EnhancedActionEvents|EnhancedInputActionIA_Jump
  (params (ActionValue :type Boolean) (ElapsedSeconds :type Float%20%28double-precision%29) (TriggeredSeconds :type Float%20%28double-precision%29) (InputAction :type Input%20Action%20Object%20Reference :default "/Game/Game/Blueprints/Input/IA_Jump.IA_Jump"))
  (:Triggered
    (Development|PrintString (Utilities|GetDisplayName InputAction) :!label _label))
  (:Started
    (goto _label))
  (:Ongoing
    (goto _label)))

(event Input|EnhancedActionEvents|EnhancedInputActionIA_LeftMouseButtonClicked
  (params (ActionValue :type Boolean) (ElapsedSeconds :type Float%20%28double-precision%29) (TriggeredSeconds :type Float%20%28double-precision%29) (InputAction :type Input%20Action%20Object%20Reference :default "/Game/Game/Blueprints/Input/IA_LeftMouseButtonClicked.IA_LeftMouseButtonClicked"))
  (:Triggered
    (bind _asplayer_controller (Utilities|Casting|CastToPlayerController (Pawn|GetController)))
    ;[1 1 1] Comment
    (Variables|/Script/Engine.PlayerController|SetbShowMouseCursor _asplayer_controller true)
    (if (.ReturnValue (Class|PlayerController|GetHitResultUnderCursorforObjects _asplayer_controller (Utilities|Array|MakeArray "ObjectTypeQuery4" "ObjectTypeQuery1") true))
      (Utilities|IsValid (.hitactor (.HitResult (Class|PlayerController|GetHitResultUnderCursorforObjects _asplayer_controller (Utilities|Array|MakeArray "ObjectTypeQuery4" "ObjectTypeQuery1") true)))
        (:Is%20Valid
          (Development|PrintString (Utilities|String|ToString(Text) (Utilities|Text|FormatText "Has tag agent: {Agent}, all tags {Tags}" (Actor|ActorHasTag (.hitactor (.HitResult (Class|PlayerController|GetHitResultUnderCursorforObjects _asplayer_controller (Utilities|Array|MakeArray "ObjectTypeQuery4" "ObjectTypeQuery1") true))) "Agent") (Utilities|Array|Get(acopy) (Variables|/Script/Engine.Actor|GetTags (.hitactor (.HitResult (Class|PlayerController|GetHitResultUnderCursorforObjects _asplayer_controller (Utilities|Array|MakeArray "ObjectTypeQuery4" "ObjectTypeQuery1") true))))))))
          (if (Actor|ActorHasTag (.hitactor (.HitResult (Class|PlayerController|GetHitResultUnderCursorforObjects _asplayer_controller (Utilities|Array|MakeArray "ObjectTypeQuery4" "ObjectTypeQuery1") true))) "Agent")
            (bind _asbp_agent (Utilities|Casting|CastToBP_Agent (.hitactor (.HitResult (Class|PlayerController|GetHitResultUnderCursorforObjects _asplayer_controller (Utilities|Array|MakeArray "ObjectTypeQuery4" "ObjectTypeQuery1") true)))))
            (Variables|Default|SetSelectedAgent _asbp_agent)
            ;[1 1 1] If both are valid then run the tree.
            ; If implemented load the tree associated with the assigned building.
            (if (and (Utilities|IsValid (Variables|Default|GetSelectedAgent)) (Utilities|IsValid (Variables|Default|GetSelectedBuilding))) :!label _label
              (Default|Assign (Variables|Default|GetSelectedAgent) (Variables|Default|GetSelectedBuilding)))
            (elif (Actor|ActorHasTag (.hitactor (.HitResult (Class|PlayerController|GetHitResultUnderCursorforObjects _asplayer_controller (Utilities|Array|MakeArray "ObjectTypeQuery4" "ObjectTypeQuery1") true))) "Building")
              (bind _asbp_building_base (Utilities|Casting|CastToBP_BuildingBase (.hitactor (.HitResult (Class|PlayerController|GetHitResultUnderCursorforObjects _asplayer_controller (Utilities|Array|MakeArray "ObjectTypeQuery4" "ObjectTypeQuery1") true)))))
              (Variables|Default|SetSelectedBuilding _asbp_building_base)
              (goto _label)
              (else
                (Utilities|IsValid (AI|GetBlackboard (AI|GetAIController (Variables|Default|GetSelectedAgent))) :!label _label_2
                  (:Is%20Valid
                    (AI|Components|Blackboard|SetValueasBool (AI|GetBlackboard (AI|GetAIController (Variables|Default|GetSelectedAgent))) (Utilities|Name|MakeLiteralName "IsAssignedKey") false)
                    (AI|Components|Blackboard|SetValueasObject (AI|GetBlackboard (AI|GetAIController (Variables|Default|GetSelectedAgent))) (Utilities|Name|MakeLiteralName "BuildingKey") 0))
                  (:Is%20Not%20Valid
                    _))
                (Variables|Default|SetSelectedAgent 0)
                (Variables|Default|SetSelectedBuilding 0)
                (Development|PrintString "Cleared selected.")))))
        (:Is%20Not%20Valid
          (goto _label_2)))
      (else
        (goto _label_2)))))

(event EventBeginPlay
  (bind _asbp_player_controller (Utilities|Casting|CastToBP_PlayerController (Game|GetPlayerController 0)))
  (Utilities|IsValid (PlayerController|LocalPlayerSubsystems|GetEnhancedInputLocalPlayerSubsystem _asbp_player_controller)
    (:Is%20Valid
      (Input|AddMappingContext (PlayerController|LocalPlayerSubsystems|GetEnhancedInputLocalPlayerSubsystem _asbp_player_controller) "/Game/Game/Blueprints/Input/IMC_Default.IMC_Default" 0 "(bIgnoreAllPressedKeysUntilRelease=True,bForceImmediately=False)"))
    (:Is%20Not%20Valid
      (Development|PrintString "Invalid local subsystem!!!"))))

(event EventTick
  (params (DeltaSeconds :type Float%20%28single-precision%29)))

(event Collision|EventActorBeginOverlap
  (params (OtherActor :type Actor%20Object%20Reference)))

(fn ConstructionScript)