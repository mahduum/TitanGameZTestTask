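; BP_Agent_V2 is an AI-controlled agent that can be assigned to and unassigned from a building through its controller's blackboard.
; On BeginPlay it stores its location as RestLocationKey, while Assignto and Unassign set or clear BuildingKey and IsAssigned checks that key's validity.
; ChangeColor writes a random Agent_Color to the M_Param_Agent parameter collection, so the color is shared rather than per agent.
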(event EventChangeColor
  (Rendering|Material|SetVectorParameterValue "/Game/MyMaterials/M_Param_Agent.M_Param_Agent" "Agent_Color" (Math|Color|MakeColor (Math|Random|RandomFloat) (Math|Random|RandomFloat) (Math|Random|RandomFloat)) :!class /Script/Engine.KismetMaterialLibrary))

(event EventUnassign
  (AI|Components|Blackboard|SetValueasObject (AI|GetBlackboard (AI|GetAIController self)) (Utilities|Name|MakeLiteralName "BuildingKey") 0))

(event EventBeginPlay
  (bind _self self)
  (AI|Components|Blackboard|SetValueasVector (AI|GetBlackboard (AI|GetAIController _self)) (Utilities|Name|MakeLiteralName "RestLocationKey") (Transformation|GetActorLocation _self)))

(event EventAssignto
  (params (Actor :type Actor%20Object%20Reference))
  (AI|Components|Blackboard|SetValueasObject (AI|GetBlackboard (AI|GetAIController self)) (Utilities|Name|MakeLiteralName "BuildingKey") Actor))

(fn ConstructionScript)

(fn IsAssigned
  (return (Utilities|IsValid (AI|Components|Blackboard|GetValueasObject (Variables|/Script/AIModule.AIController|GetBlackboard (AI|GetAIController self)) (Utilities|Name|MakeLiteralName "BuildingKey")))))