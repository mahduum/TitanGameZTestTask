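; Test game mode that sets up the root UI layer and caches key test actors at BeginPlay.
; It creates and activates a UI_Layer widget, with AddUI and RemoveUI events that add and remove activatable widgets on its stack.
; As a temporary stand-in for click selection, it caches the first agent and first building of types A, B and C, each lookup nested inside the previous one's success.
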(event EventBeginPlay
  (Utilities|FlowControl|Sequence
    (:then_0
      (bind _returnvalue (UserInterface|CreateWidget "/Game/Game/UI/UI_Layer.UI_Layer_C"))
      (UserInterface|Viewport|AddtoViewport _returnvalue 0)
      (bind _output_get (Variables|Default|SetUI%20HUD _returnvalue))
      (Class|CommonActivatableWidget|ActivateWidget _output_get))
    (:then_1
      ;[1 1 1] Temporary way of finding and caching main actors for test purposes. Normally a point and click selection would be used.
      (bind _outactors (Actor|GetAllActorsOfClass "/Game/Game/Blueprints/Agents/BP_Agent_V2.BP_Agent_V2_C"))
      (if (Utilities|Array|IsNotEmpty _outactors)
        (Variables|Default|SetAgent (Utilities|Array|Get(acopy) _outactors))
        (bind _outactors_2 (Actor|GetAllActorsOfClass "/Game/Game/Blueprints/Buildings/BP_Building_A.BP_Building_A_C"))
        (if (Utilities|Array|IsNotEmpty _outactors_2)
          (Variables|Default|SetBuilding_A (Utilities|Array|Get(acopy) _outactors_2))
          (bind _outactors_3 (Actor|GetAllActorsOfClass "/Game/Game/Blueprints/Buildings/BP_Building_B.BP_Building_B_C"))
          (if (Utilities|Array|IsNotEmpty _outactors_3)
            (Variables|Default|SetBuilding_B (Utilities|Array|Get(acopy) _outactors_3))
            (bind _outactors_4 (Actor|GetAllActorsOfClass "/Game/Game/Blueprints/Buildings/BP_Building_C.BP_Building_C_C"))
            (if (Utilities|Array|IsNotEmpty _outactors_4)
              (Variables|Default|SetBuilding_C (Utilities|Array|Get(acopy) _outactors_4)))))))))

(event EventAddUI
  (params (ActivatableWidgetClass :type Common%20Activatable%20Widget%20Class%20Reference))
  (Default|AddStackItem (Variables|Default|GetUI%20HUD) ActivatableWidgetClass))

(event EventRemoveUI
  (Default|RemoveStackItem (Variables|Default|GetUI%20HUD)))

(fn ConstructionScript)